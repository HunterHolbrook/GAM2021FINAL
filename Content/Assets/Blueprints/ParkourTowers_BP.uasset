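; Parkour towers Blueprint that moves six cube components into their end positions when ActivateTowers is called.
; A Sequence starts one timeline per cube, with progressively longer delays staggering the movements into a cascade.
; Each update lerps from the cube's current relative location, rather than a stored start, toward its TowerEnd variable, so the timeline alpha compounds.
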(event `ActivateTowers`
  (`|ExecutionSequence`
    (:`then_0`
      (bind (_direction _newtrack_0) (`Timeline|TowerActivation`)
        (:`Update`
          (`SceneComponent.K2_SetRelativeLocation` (`self.Cube`) (`KismetMathLibrary.VLerp` (`SceneComponent.RelativeLocation` (`self.Cube`)) (`self.Tower1End`) _newtrack_0) false false))))
    (:`then_1`
      (`KismetSystemLibrary.Delay` 0.5)
      (bind (_direction_2 _newtrack_0_2) (`Timeline|Timeline_0`)
        (:`Update`
          (`SceneComponent.K2_SetRelativeLocation` (`self.Cube1`) (`KismetMathLibrary.VLerp` (`SceneComponent.RelativeLocation` (`self.Cube1`)) (`self.Tower2End`) _newtrack_0_2) false false))))
    (:`then_2`
      (`KismetSystemLibrary.Delay` 1.0)
      (bind (_direction_3 _newtrack_0_3) (`Timeline|Timeline_1`)
        (:`Update`
          (`SceneComponent.K2_SetRelativeLocation` (`self.Cube2`) (`KismetMathLibrary.VLerp` (`SceneComponent.RelativeLocation` (`self.Cube2`)) (`self.Tower3End`) _newtrack_0_3) false false))))
    (:`then_3`
      (`KismetSystemLibrary.Delay` 1.5)
      (bind (_direction_4 _newtrack_0_4) (`Timeline|Timeline_2`)
        (:`Update`
          (`SceneComponent.K2_SetRelativeLocation` (`self.Cube3`) (`KismetMathLibrary.VLerp` (`SceneComponent.RelativeLocation` (`self.Cube3`)) (`self.Tower4End`) _newtrack_0_4) false false))))
    (:`then_4`
      (`KismetSystemLibrary.Delay` 2.0)
      (bind (_direction_5 _newtrack_0_5) (`Timeline|Timeline_3`)
        (:`Update`
          (`SceneComponent.K2_SetRelativeLocation` (`self.Cube4`) (`KismetMathLibrary.VLerp` (`SceneComponent.RelativeLocation` (`self.Cube4`)) (`self.Tower5End`) _newtrack_0_5) false false))))
    (:`then_5`
      (`KismetSystemLibrary.Delay` 2.5)
      (bind (_direction_6 _newtrack_0_6) (`Timeline|Timeline_4`)
        (:`Update`
          (`SceneComponent.K2_SetRelativeLocation` (`self.Cube5`) (`KismetMathLibrary.VLerp` (`SceneComponent.RelativeLocation` (`self.Cube5`)) (`self.Tower6End`) _newtrack_0_6) false false))))))

(fn `UserConstructionScript`)