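; A moving platform Blueprint whose Cube travels along its local X axis after something overlaps its Collision component.
; The overlap passes a DoOnce, waits briefly, then plays the ElevatorMove timeline, which lerps the Cube from its current position toward an X offset on each update.
; Tick watches NeedToResetPlatform, which this file only clears, to stop the timeline, restore the BeginPlay location and re-arm the DoOnce.
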(event `self.ReceiveBeginPlay`
  (set `self.MovingPlatformStartLocation` (`SceneComponent.RelativeLocation` (`self.Cube`))))

(event `self.ReceiveTick`
  (params (DeltaSeconds :type "Float (single-precision)"))
  (if (`self.NeedToResetPlatform`)
    (`|ExecutionSequence`
      (:`then_0`
        (bind (_direction _newtrack_1) (`Timeline|ElevatorMove` :!via `Stop` :!label _label)
          (:`Update`
            (`SceneComponent.K2_SetRelativeLocation` (`self.Cube`) (`KismetMathLibrary.VLerp` (`SceneComponent.RelativeLocation` (`self.Cube`)) (+ (`SceneComponent.RelativeLocation` (`self.Cube`)) (30.049999 0.0 0.0)) _newtrack_1) false false))))
      (:`then_1`
        (`SceneComponent.K2_SetRelativeLocation` (`self.Cube`) (`self.MovingPlatformStartLocation`) false false)
        (set `self.NeedToResetPlatform` false))
      (:`then_2`
        (goto _label_2 :!via `Reset`)))))

(event `self.Collision.OnComponentBeginOverlap`
  (params (OverlappedComponent :type "PrimitiveComponent Object Reference") (OtherActor :type "Actor Object Reference") (OtherComp :type "PrimitiveComponent Object Reference") (OtherBodyIndex :type Integer) (bFromSweep :type Boolean) (SweepResult :type "HitResult Structure (by ref)"))
  (`/Engine/EditorBlueprintResources/StandardMacros.DoOnce` false :!label _label_2
    (:`Completed`
      (`KismetSystemLibrary.Delay` 0.5)
      (goto _label :!via `PlayFromStart`))))

(fn `UserConstructionScript`)