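; Door actor, named as a post-obstacle door, that lowers and raises a Cube through two trigger volumes.
; Overlapping Collision plays a timeline that lowers the Cube, and overlapping Collision1 plays another that raises it, each gated by a DoOnce.
; ResetDoorOpen re-arms both gates.
; Each timeline update lerps from the Cube's current location toward a Z offset, so movement accumulates instead of following fixed endpoints.
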(event `self.Collision.OnComponentBeginOverlap`
  (params (OverlappedComponent :type "PrimitiveComponent Object Reference") (OtherActor :type "Actor Object Reference") (OtherComp :type "PrimitiveComponent Object Reference") (OtherBodyIndex :type Integer) (bFromSweep :type Boolean) (SweepResult :type "HitResult Structure (by ref)"))
  (`/Engine/EditorBlueprintResources/StandardMacros.DoOnce` false :!label _label
    (:`Completed`
      (bind (_direction _newtrack_0) (`Timeline|DoorOpen`)
        (:`Update`
          (`SceneComponent.K2_SetWorldLocation` (`self.Cube`) (`KismetMathLibrary.VLerp` (`SceneComponent.K2_GetComponentLocation` (`self.Cube`)) (- (`SceneComponent.K2_GetComponentLocation` (`self.Cube`)) (0.0 0.0 3.25)) _newtrack_0) false false))))))

(event `ResetDoorOpen`
  (`|ExecutionSequence`
    (:`then_0`
      (goto _label :!via `Reset`))
    (:`then_1`
      (goto _label_2 :!via `Reset`))))

(event `self.Collision1.OnComponentBeginOverlap`
  (params (OverlappedComponent :type "PrimitiveComponent Object Reference") (OtherActor :type "Actor Object Reference") (OtherComp :type "PrimitiveComponent Object Reference") (OtherBodyIndex :type Integer) (bFromSweep :type Boolean) (SweepResult :type "HitResult Structure (by ref)"))
  (`/Engine/EditorBlueprintResources/StandardMacros.DoOnce` false :!label _label_2
    (:`Completed`
      (bind (_direction _newtrack_0) (`Timeline|Timeline_0`)
        (:`Update`
          (`SceneComponent.K2_SetWorldLocation` (`self.Cube`) (`KismetMathLibrary.VLerp` (`SceneComponent.K2_GetComponentLocation` (`self.Cube`)) (+ (`SceneComponent.K2_GetComponentLocation` (`self.Cube`)) (0.0 0.0 3.25)) _newtrack_0) false false))))))

(fn `UserConstructionScript`)