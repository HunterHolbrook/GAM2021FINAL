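; Elevator actor that moves itself 5000 units along its X axis when something begins overlapping its Collision component.
; Each overlap sets an end location relative to the root's current position, waits half a second, then plays the ElevatorMove timeline.
; The timeline lerps from the root's current, continually updated location rather than a stored start, so motion compounds toward the target.
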(event `self.Collision.OnComponentBeginOverlap`
  (params (OverlappedComponent :type "PrimitiveComponent Object Reference") (OtherActor :type "Actor Object Reference") (OtherComp :type "PrimitiveComponent Object Reference") (OtherBodyIndex :type Integer) (bFromSweep :type Boolean) (SweepResult :type "HitResult Structure (by ref)"))
  (bind _output_get (set `self.ElevatorEndLocation` (+ (`SceneComponent.RelativeLocation` (`self.DefaultSceneRoot`)) (5000.0 0.0 0.0))))
  (`KismetSystemLibrary.Delay` 0.5)
  (bind (_direction _newtrack_0) (`Timeline|ElevatorMove`)
    (:`Update`
      (`SceneComponent.K2_SetRelativeLocation` (`self.DefaultSceneRoot`) (`KismetMathLibrary.VLerp` (`SceneComponent.RelativeLocation` (`self.DefaultSceneRoot`)) _output_get _newtrack_0) false false))))

(fn `UserConstructionScript`)