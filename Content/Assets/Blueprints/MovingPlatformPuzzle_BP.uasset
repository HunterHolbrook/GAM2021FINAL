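; Puzzle platform actor that floats from BeginPlay and can be lowered or moved to set end positions.
; PlatformFloat timeline offsets the actor each update until LowerPlatform, gated to run once, stops it and lowers Platform after a short delay.
; Any Collision overlap starts a delayed move toward MovedPlatformEnd, as the character-name check is unused.
; Both moves lerp from the current relative location each update, so steps compound.
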(event `self.ReceiveBeginPlay`
  (bind (_direction _movement) (`Timeline|PlatformFloat` :!label _label)
    (:`Update`
      (`self.K2_AddActorLocalOffset` _movement))))

(event `LowerPlatform`
  (`/Engine/EditorBlueprintResources/StandardMacros.DoOnce` false
    (:`Completed`
      (`|ExecutionSequence`
        (:`then_0`
          (goto _label :!via `Stop`))
        (:`then_1`
          (`KismetSystemLibrary.Delay` 0.5)
          (bind (_direction _newtrack_1) (`Timeline|LowerPlatformAnim`)
            (:`Update`
              (`SceneComponent.K2_SetRelativeLocation` (`self.Platform`) (`KismetMathLibrary.VLerp` (`SceneComponent.RelativeLocation` (`self.Platform`)) (`self.LoweredPlatformEnd`) _newtrack_1) false false))))))))

(event `self.Collision.OnComponentBeginOverlap`
  (params (OverlappedComponent :type "PrimitiveComponent Object Reference") (OtherActor :type "Actor Object Reference") (OtherComp :type "PrimitiveComponent Object Reference") (OtherBodyIndex :type Integer) (bFromSweep :type Boolean) (SweepResult :type "HitResult Structure (by ref)"))
  (`KismetSystemLibrary.Delay` 1.0)
  (bind (_direction _newtrack_0) (`Timeline|PlatformMoveAnim`)
    (:`Update`
      (`SceneComponent.K2_SetRelativeLocation` (`self.Platform`) (`KismetMathLibrary.VLerp` (`SceneComponent.RelativeLocation` (`self.Platform`)) (`self.MovedPlatformEnd`) _newtrack_0) false false))))

(fn `UserConstructionScript`)