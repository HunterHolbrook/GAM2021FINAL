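; Enemy AI Blueprint that chases the player, trades damage on overlap, and ends the game when it dies.
; Pawn sensing starts an AI move, then after a delay a timeline lerps the enemy toward the player's stored location.
; Collision overlaps drain player health, or enemy health after a delay for projectiles.
; Tick checks enemy health for exactly zero, then destroys the actor, disables input and issues a delayed quit.
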(event `self.PawnSensing.OnSeePawn`
  (params (Pawn :type "Pawn Object Reference"))
  ;[1 1 1] EnemyMovement
  (bind _asfirst_person_character (cast `/Game/FirstPersonBP/Blueprints/FirstPersonCharacter` Pawn))
  (`|AIMoveTo` self (0.0 0.0 0.0) _asfirst_person_character
    (:`then`
      (`KismetSystemLibrary.Delay` 3.0)
      (bind (_direction _newtrack_0) (`Timeline|Timeline_0` :!via `PlayFromStart`)
        (:`Update`
          (`self.K2_SetActorLocation` (`KismetMathLibrary.VLerp` (`SceneComponent.K2_GetComponentLocation` (`self.CapsuleComponent`)) (`/Game/FirstPersonBP/Blueprints/FirstPersonCharacter.PlayerLocation` _asfirst_person_character) _newtrack_0)))))))

(event `self.Collision.OnComponentBeginOverlap`
  (params (OverlappedComponent :type "PrimitiveComponent Object Reference") (OtherActor :type "Actor Object Reference") (OtherComp :type "PrimitiveComponent Object Reference") (OtherBodyIndex :type Integer) (bFromSweep :type Boolean) (SweepResult :type "HitResult Structure (by ref)"))
  ;[1 1 1] LoseHealthOnEnemyHit
  (`|ExecutionSequence`
    (:`then_0`
      (bind _asfirst_person_character (cast `/Game/FirstPersonBP/Blueprints/FirstPersonCharacter` OtherActor))
      (set `/Game/FirstPersonBP/Blueprints/FirstPersonCharacter.Health` (- (`/Game/FirstPersonBP/Blueprints/FirstPersonCharacter.Health` _asfirst_person_character) 0.1) _asfirst_person_character))
    (:`then_1`
      ;[1 1 1] Enemy Loses Health When Hit
      (`KismetSystemLibrary.Delay` 3.0)
      (cast `/Game/FirstPersonBP/Blueprints/FirstPersonProjectile` OtherActor)
      (set `self.EnemyHealth` (- (`self.EnemyHealth`) 0.02))
      (`KismetSystemLibrary.PrintString` (`KismetStringLibrary.Conv_DoubleToString` (`self.EnemyHealth`))))))

(event `self.ReceiveTick`
  (params (DeltaSeconds :type "Float (single-precision)"))
  ;[1 1 1] If Enemy Dies, Game Over
  (if (== (`self.EnemyHealth`) 0.0)
    (`self.K2_DestroyActor`)
    (`self.DisableInput` (`GameplayStatics.GetPlayerCharacter` 0) (`GameplayStatics.GetPlayerController` 0))
    (`KismetSystemLibrary.Delay` 2.0)
    (`KismetSystemLibrary.QuitGame` null "Quit")))

(fn `UserConstructionScript`)